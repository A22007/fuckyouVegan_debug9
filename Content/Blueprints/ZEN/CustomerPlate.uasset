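; CustomerPlate is an unfinished customer plate Blueprint that sets a customer's order and creates a Hukidasi widget.
; BeginPlay picks Order from OrderItems by random index, though the range currently allows only the first entry, then creates the widget without further setup.
; The Box overlap event switches on Order with no actions attached, and leftover debug print and comparison nodes never run.
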(event OnComponentBeginOverlap(Box)
  (params (OverlappedComponent :type Primitive%20Component%20Object%20Reference) (OtherActor :type Actor%20Object%20Reference) (OtherComp :type Primitive%20Component%20Object%20Reference) (OtherBodyIndex :type Integer) (bFromSweep :type Boolean) (SweepResult :type Hit%20Result%20Structure%20%28by%20ref%29))
  (switch string (Variables|Default|GetOrder)))

(event EventBeginPlay
  ;[1 1 1] オーダーをランダムに決める
  (Variables|Default|SetOrder (Utilities|Array|Get(acopy) (Variables|Default|GetOrderItems) (Math|Random|RandomIntegerinRange 0 0)))
  (UserInterface|CreateWidget "/Game/widget/Hukidasi.Hukidasi_C"))

(event Collision|EventActorBeginOverlap
  (params (OtherActor :type Actor%20Object%20Reference)))

(event EventTick
  (params (DeltaSeconds :type Float%20%28single-precision%29)))

(fn ConstructionScript)