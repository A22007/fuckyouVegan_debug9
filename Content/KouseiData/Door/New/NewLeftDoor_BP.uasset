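; Blueprint for an automatic double door that swings open when something overlaps its Box and closes when the overlap ends.
; Separate open and close timelines lerp the relative yaw of the left and right door components in opposite directions.
; Each timeline stops the other and starts from its last stored angle, so the swing can reverse midway.
; A debug "Hello" prints when opening finishes.
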(event OnComponentEndOverlap(Box)
  (params (OverlappedComponent :type Primitive%20Component%20Object%20Reference) (OtherActor :type Actor%20Object%20Reference) (OtherComp :type Primitive%20Component%20Object%20Reference) (OtherBodyIndex :type Integer))
  (bind _新規track_0 (Timeline|タイムライン_1 PlayFromStart)
    (:Update
      (bind _output_get (Variables|Default|SetCloseLeft (Math|Float|Lerp (Variables|Default|GetOpenLeft) 0.0 _新規track_0)))
      (Transformation|SetRelativeRotation (Variables|Default|GetLeftDoor_New) (Math|Rotator|MakeRotator 0.0 0.0 _output_get) false false)
      (bind _output_get_2 (Variables|Default|SetCloseRight (Math|Float|Lerp (Variables|Default|GetOpenRight) 0.0 _新規track_0)))
      (Transformation|SetRelativeRotation (Variables|Default|GetNewRightDoor_BP) (Math|Rotator|MakeRotator 0.0 0.0 _output_get_2) false false)
      (bind _新規track_0_2 (Timeline|タイムライン Stop)
        (:Update
          (bind _output_get_3 (Variables|Default|SetOpenLeft (Math|Float|Lerp (Variables|Default|GetCloseLeft) 1.2e+02 _新規track_0_2)))
          (Transformation|SetRelativeRotation (Variables|Default|GetLeftDoor_New) (Math|Rotator|MakeRotator 0.0 0.0 _output_get_3) false false)
          (bind _output_get_4 (Variables|Default|SetOpenRight (Math|Float|Lerp (Variables|Default|GetCloseRight) -1.2e+02 _新規track_0_2)))
          (Transformation|SetRelativeRotation (Variables|Default|GetNewRightDoor_BP) (Math|Rotator|MakeRotator 0.0 0.0 _output_get_4) false false)
          (Timeline|タイムライン_1 Stop))
        (:Finished
          (Development|PrintString "Hello"))))))

(event OnComponentBeginOverlap(Box)
  (params (OverlappedComponent :type Primitive%20Component%20Object%20Reference) (OtherActor :type Actor%20Object%20Reference) (OtherComp :type Primitive%20Component%20Object%20Reference) (OtherBodyIndex :type Integer) (bFromSweep :type Boolean) (SweepResult :type Hit%20Result%20Structure%20%28by%20ref%29))
  (bind _新規track_0 (Timeline|タイムライン PlayFromStart)
    (:Update
      (bind _output_get (Variables|Default|SetOpenLeft (Math|Float|Lerp (Variables|Default|GetCloseLeft) 1.2e+02 _新規track_0)))
      (Transformation|SetRelativeRotation (Variables|Default|GetLeftDoor_New) (Math|Rotator|MakeRotator 0.0 0.0 _output_get) false false)
      (bind _output_get_2 (Variables|Default|SetOpenRight (Math|Float|Lerp (Variables|Default|GetCloseRight) -1.2e+02 _新規track_0)))
      (Transformation|SetRelativeRotation (Variables|Default|GetNewRightDoor_BP) (Math|Rotator|MakeRotator 0.0 0.0 _output_get_2) false false)
      (bind _新規track_0_2 (Timeline|タイムライン_1 Stop)
        (:Update
          (bind _output_get_3 (Variables|Default|SetCloseLeft (Math|Float|Lerp (Variables|Default|GetOpenLeft) 0.0 _新規track_0_2)))
          (Transformation|SetRelativeRotation (Variables|Default|GetLeftDoor_New) (Math|Rotator|MakeRotator 0.0 0.0 _output_get_3) false false)
          (bind _output_get_4 (Variables|Default|SetCloseRight (Math|Float|Lerp (Variables|Default|GetOpenRight) 0.0 _新規track_0_2)))
          (Transformation|SetRelativeRotation (Variables|Default|GetNewRightDoor_BP) (Math|Rotator|MakeRotator 0.0 0.0 _output_get_4) false false)
          (Timeline|タイムライン Stop))))
    (:Finished
      (Development|PrintString "Hello"))))

(event EventBeginPlay)

(event Collision|EventActorBeginOverlap
  (params (OtherActor :type Actor%20Object%20Reference)))

(event EventTick
  (params (DeltaSeconds :type Float%20%28single-precision%29)))

(fn ConstructionScript)